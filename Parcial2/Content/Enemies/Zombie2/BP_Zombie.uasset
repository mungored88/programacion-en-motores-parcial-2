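; Zombie enemy that chases the player character and stops moving once its health is depleted.
; Tick calls WidgetLookCam and, while alive, reissues AIMoveTo toward BP_My_Character_In_C_ok every frame.
; On arrival it plays a sound at the mesh and clears ParamWalk on BP_Zombie2Animation for a second before restoring it.
; BeginPlay defers to the parent, while the parent Tick call is left unconnected.
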(event EventBeginPlay
  (|CallParentFunction))

(event Collision|EventActorBeginOverlap
  (params (OtherActor :type Actor%20Object%20Reference)))

(event EventTick
  (params (DeltaSeconds :type Float%20%28single-precision%29))
  (CallFunction|WidgetLookCam)
  (if (> (Variables|Default|GetHealth) 0.1)
    (bind _returnvalue (Actor|GetActorOfClass "/Game/Blueprints/BP_My_Character_In_C_ok.BP_My_Character_In_C_ok_C"))
    (AI|AIMoveTo self (Transformation|GetActorLocation _returnvalue) 0 (Variables|Default|GetDistance) false
      (:OnSuccess
        (Audio|SpawnSoundatLocation 0 (Transformation|GetWorldLocation (Variables|Character|GetMesh)) "0, 0, 0" 0.15 1.0 0.0 0 0)
        (bind _asbp_zombie_2animation (Utilities|Casting|CastToBP_Zombie2Animation (Components|SkeletalMesh|GetAnimInstance (Variables|Character|GetMesh))))
        (Variables|/Game/Enemies/Zombie2/BP_Zombie2Animation.BP_Zombie2Animation_C|SetParamWalk _asbp_zombie_2animation false)
        (Utilities|FlowControl|Delay 1.0)
        (Variables|/Game/Enemies/Zombie2/BP_Zombie2Animation.BP_Zombie2Animation_C|SetParamWalk _asbp_zombie_2animation true)))
    (else
      (Components|Movement|StopMovementImmediately (Variables|Character|GetCharacterMovement)))))

(fn ConstructionScript
  (|CallParentFunction))