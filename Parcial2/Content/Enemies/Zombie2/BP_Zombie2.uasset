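; Zombie enemy that chases the player character and awards points on death.
; Tick turns its life bar toward the camera and reissues AIMoveTo; arrival plays a sound and pauses the animation's walk flag for a second.
; Damage updates the bar; at zero health the mesh ragdolls, then after a delay the score rises and the actor is randomly destroyed or left.
; GenerationHit spawns a BP_Hit_Damage actor carrying its attack damage.
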(event Custom|Damage
  (params (DamageAmount :type Float%20%28single-precision%29))
  (bind _output_get (Variables|Components|SetHealth (Math|Float|Clamp(Float) (- (Variables|Components|GetHealth) DamageAmount) 0.0 1e+02)))
  (bind _asui_life_enemy (Utilities|Casting|CastToUI_Life_Enemy (UserInterface|GetWidget (Variables|Default|GetWidget_Life_Enemy))))
  (Default|UpdateLife _asui_life_enemy (Variables|Components|GetHealth) 1e+02)
  (if (== _output_get 0.0)
    (Class|SkeletalMeshComponent|SetAllBodiesSimulatePhysics (Variables|Character|GetMesh) true)
    (Collision|SetCollisionEnabled (Variables|Collision|GetCapsuleComponent) "NoCollision")
    (Collision|SetCollisionEnabled (Variables|Character|GetMesh) "QueryAndPhysics")
    (Utilities|FlowControl|Delay 2.0)
    (bind _returnvalue (Actor|GetActorOfClass "/Game/Blueprints/BP_My_Character_In_C_ok.BP_My_Character_In_C_ok_C"))
    (bind _asbp_my_character_in_c_ok (Utilities|Casting|CastToBP_My_Character_In_C_ok _returnvalue))
    (bind _output_get_2 (Variables|/Game/Blueprints/BP_My_Character_In_C_ok.BP_My_Character_In_C_ok_C|SetPoints _asbp_my_character_in_c_ok (+ (Variables|/Game/Blueprints/BP_My_Character_In_C_ok.BP_My_Character_In_C_ok_C|GetPoints _asbp_my_character_in_c_ok) 500)))
    (Default|UpdateScore (Variables|/Game/Blueprints/BP_My_Character_In_C_ok.BP_My_Character_In_C_ok_C|GetUIPlayer _asbp_my_character_in_c_ok) _output_get_2)
    (if (not (== (Math|Random|RandomIntegerinRange 0 2) 1))
      (Actor|DestroyActor))))

(event EventBeginPlay
  (Variables|/Script/Engine.CharacterMovementComponent|SetMaxWalkSpeed (Variables|Character|GetCharacterMovement) (Variables|Components|GetMaxSpeed)))

(event EventTick
  (params (DeltaSeconds :type Float%20%28single-precision%29))
  (CallFunction|WidgetLookCam)
  (if (> (Variables|Components|GetHealth) 0.1)
    (bind _returnvalue (Actor|GetActorOfClass "/Game/Blueprints/BP_My_Character_In_C_ok.BP_My_Character_In_C_ok_C"))
    (AI|AIMoveTo self (Transformation|GetActorLocation _returnvalue) 0 (Variables|Components|GetDistance) false
      (:OnSuccess
        (Audio|SpawnSoundatLocation 0 (Transformation|GetWorldLocation (Variables|Character|GetMesh)) "0, 0, 0" 0.15 1.0 0.0 0 0)
        (bind _asbp_zombie_2animation (Utilities|Casting|CastToBP_Zombie2Animation (Components|SkeletalMesh|GetAnimInstance (Variables|Character|GetMesh))))
        (Variables|/Game/Enemies/Zombie2/BP_Zombie2Animation.BP_Zombie2Animation_C|SetParamWalk _asbp_zombie_2animation false)
        (Utilities|FlowControl|Delay 1.0)
        (Variables|/Game/Enemies/Zombie2/BP_Zombie2Animation.BP_Zombie2Animation_C|SetParamWalk _asbp_zombie_2animation true)))
    (else
      (Components|Movement|StopMovementImmediately (Variables|Character|GetCharacterMovement)))))

(fn ConstructionScript)

(fn WidgetLookCam
  (Transformation|SetWorldRotation (Variables|Default|GetWidget_Life_Enemy) (Math|Rotator|MakeRotator 0.0 0.0 (.Yaw (Math|Rotator|BreakRotator (Math|Rotator|FindLookatRotation (Transformation|GetWorldLocation (Variables|Default|GetWidget_Life_Enemy)) (Camera|GetCameraLocation (Game|GetPlayerCameraManager 0)))))) false false))

(fn GenerationHit
  (bind _hit (Variables|Default|GetHit))
  (bind _returnvalue (Game|SpawnActorfromClass "/Game/Blueprints/BP_Hit_Damage.BP_Hit_Damage_C" (Math|Transform|MakeTransform (Transformation|GetWorldLocation _hit) (Transformation|GetWorldRotation _hit) "1,1,1") "Undefined" 0 0))
  (Variables|/Game/Blueprints/BP_Hit_Damage.BP_Hit_Damage_C|SetDamages _returnvalue (Variables|Components|GetDamageAplicateInPlayer)))