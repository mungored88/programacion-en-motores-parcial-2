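; Player character Blueprint for a zombie shooter, handling gun fire, health, pausing, jump animation and switch interaction.
; Shots line-trace from the gun point, using a magazine count and difficulty-based bullet damage on BP_Zombie1; the reload logic is disconnected.
; Ammo and damage update the score/life widget, while a Tick death check shows mission failed, then loads the menu after a delay.
; Capsule overlaps track simple or multiple switches for the Action input.
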(event OnComponentBeginOverlap(CapsuleComponent)
  (params (OverlappedComponent :type Primitive%20Component%20Object%20Reference) (OtherActor :type Actor%20Object%20Reference) (OtherComp :type Primitive%20Component%20Object%20Reference) (OtherBodyIndex :type Integer) (bFromSweep :type Boolean) (SweepResult :type Hit%20Result%20Structure%20%28by%20ref%29))
  ;[1 1 1] Switches
  (bind _assimple_switch (Utilities|Casting|CastToSimple_switch OtherActor)
    (:then
      (Variables|Default|SetAs%20Switch%20Select _assimple_switch))
    (:CastFailed
      (bind _asmultiple_switch (Utilities|Casting|CastToMultiple_Switch OtherActor))
      (Variables|Default|SetMultibple%20switch _asmultiple_switch))))

(event OnComponentEndOverlap(CapsuleComponent)
  (params (OverlappedComponent :type Primitive%20Component%20Object%20Reference) (OtherActor :type Actor%20Object%20Reference) (OtherComp :type Primitive%20Component%20Object%20Reference) (OtherBodyIndex :type Integer))
  ;[1 1 1] Switches
  (Utilities|Casting|CastToSimple_switch OtherActor
    (:then
      (Variables|Default|SetAs%20Switch%20Select 0))
    (:CastFailed
      (Utilities|Casting|CastToMultiple_Switch OtherActor)
      (Variables|Default|SetMultibple%20switch 0))))

(event Custom|Damage
  (params (Receive_damage :type Float%20%28single-precision%29))
  (bind _uiplayer (Variables|Default|GetUIPlayer))
  ;[1 0.6277 0.6509] -Receive Damage
  (Variables|Default|SetHealth (Math|Float|Clamp(Float) (- (Variables|Default|GetHealth) Receive_damage) 0.0 1e+02))
  (Default|UpdateHealth _uiplayer (Variables|Default|GetHealth))
  (Default|ShowGetDamage _uiplayer))

(event EventBeginPlay
  ;[0.1378 0.4947 1] -Create and show Score widget
  (Utilities|FlowControl|Sequence
    (:then_0
      (bind _returnvalue (UserInterface|CreateWidget "/Game/UI/UI_ScoreLife.UI_ScoreLife_C"))
      (bind _output_get (Variables|Default|SetUIPlayer _returnvalue))
      (UserInterface|Viewport|AddtoViewport _output_get 0)
      (Default|UpdateAmmo _output_get (Variables|Default|GetBulletMagazine))
      (bind _asdificultad_level_intance (Utilities|Casting|CastToDificultadLevelIntance (Game|GetGameInstance)))
      (Variables|Default|SetDañoBala (.Value (Utilities|Map|Find (Variables|Default|GetMapaDañoBala) (Variables|/Game/MenuStaff/Dificultades/DificultadLevelIntance.DificultadLevelIntance_C|GetDificultad _asdificultad_level_intance)))))
    (:then_1
      (Transformation|AttachComponentToComponent (Variables|Default|GetGun) (Variables|Character|GetMesh) "Weapon" "SnapToTarget" "KeepRelative" "KeepRelative" true))))

(event EventTick
  (params (DeltaSeconds :type Float%20%28single-precision%29))
  ;[1 0.1512 0.2878] -Is Dead?
  (CallFunction|CheckIsDead)
  (if (Variables|Default|GetIsDead)
    (Utilities|FlowControl|Delay 5.0)
    (Game|OpenLevel(byName) "Menu")))

(event Collision|EventActorBeginOverlap
  (params (OtherActor :type Actor%20Object%20Reference)))

(event Input|ActionEvents|InputActionAction
  (params (Key :type Key%20Structure :default "None"))
  (bind _as_switch_select (Variables|Default|GetAs%20Switch%20Select))
  (bind _multibple_switch (Variables|Default|GetMultibple%20switch))
  ;[1 1 1] Switches
  (:Pressed
    (Utilities|FlowControl|Sequence
      (:then_0
        (Utilities|IsValid _as_switch_select
          (:Is%20Valid
            (Default|Accionar _as_switch_select))))
      (:then_1
        (Utilities|IsValid _multibple_switch
          (:Is%20Valid
            (Default|MultiAction _multibple_switch)))))))

(event Input|MouseEvents|LeftMouseButton
  (params (Key :type Key%20Structure :default "None"))
  (bind _particle (Variables|Default|Getparticle))
  (bind _gunpoint (Variables|Default|GetGunpoint))
  (bind _returnvalue (Transformation|GetWorldLocation _gunpoint))
  ;[1 0.03438 0.02775] -Shoot
  (:Pressed
    (if (not (Variables|Default|GetIsReloading))
      ;;[1 1 1] Check Gun Magazine and Use Bullet
      (if (> (Variables|Default|GetBulletMagazine) 0)
        (Variables|Default|SetBulletMagazine (- (Variables|Default|GetBulletMagazine) 1))
        (bind _outhit (Collision|LineTraceByChannel _returnvalue (+ _returnvalue (* (Math|Vector|GetForwardVector _gunpoint) 5e+03)) "TraceTypeQuery1" false 0 "None"))
        (bind _asmy_character_in_c_anim_blueprint (Utilities|Casting|CastToMy_Character_In_C_Anim_Blueprint (Components|SkeletalMesh|GetAnimInstance (Variables|Character|GetMesh))))
        (Variables|/Game/Blueprints/My_Character_In_C_Anim_Blueprint.My_Character_In_C_Anim_Blueprint_C|SetParam_Shoot _asmy_character_in_c_anim_blueprint true)
        (Audio|SpawnSoundatLocation 0 (Transformation|GetWorldLocation _particle) "0, 0, 0" 1.0 1.0 0.0 0 0)
        (Effects|SpawnEmitteratLocation "/Game/StarterContent/Particles/P_Explosion.P_Explosion" (Transformation|GetWorldLocation _particle) "0, 0, 0" "0.050000,0.050000,0.050000")
        (Default|UpdateAmmo (Variables|Default|GetUIPlayer) (Variables|Default|GetBulletMagazine))
        (bind _asbp_zombie_1 (Utilities|Casting|CastToBP_Zombie1 (.HitActor (Collision|BreakHitResult _outhit))))
        (Default|Damage _asbp_zombie_1 (Variables|Default|GetDañoBala))
        (Effects|SpawnEmitteratLocation "/Game/FXVarietyPack/Particles/P_ky_hit2.P_ky_hit2" (.Location (Collision|BreakHitResult _outhit)) "0, 0, 0" "0.050000,0.050000,0.050000")
        (Variables|/Game/Blueprints/My_Character_In_C_Anim_Blueprint.My_Character_In_C_Anim_Blueprint_C|SetParam_Shoot _asmy_character_in_c_anim_blueprint false)))))

(event Input|KeyboardEvents|Escape
  (params (Key :type Key%20Structure :default "None"))
  (bind _returnvalue (Game|GetPlayerController 0))
  (:Pressed
    (Utilities|FlowControl|FlipFlop
      (:A
        (bind _returnvalue_2 (UserInterface|CreateWidget "/Game/MenuStaff/Pause_Menu.Pause_Menu_C"))
        (UserInterface|Viewport|AddtoViewport _returnvalue_2 0)
        (Game|SetGamePaused true)
        (Variables|/Script/Engine.PlayerController|SetbShowMouseCursor _returnvalue true))
      (:B
        (Widget|RemovefromParent _returnvalue_2)
        (Game|SetGamePaused false)
        (Variables|/Script/Engine.PlayerController|SetbShowMouseCursor _returnvalue false)))))

(event Input|KeyboardEvents|SpaceBar
  (params (Key :type Key%20Structure :default "None"))
  ;[0.675 0.3368 1] -Jump
  (:Pressed
    (bind _asmy_character_in_c_anim_blueprint (Utilities|Casting|CastToMy_Character_In_C_Anim_Blueprint (Components|SkeletalMesh|GetAnimInstance (Variables|Character|GetMesh))))
    (Variables|/Game/Blueprints/My_Character_In_C_Anim_Blueprint.My_Character_In_C_Anim_Blueprint_C|SetParam_Jump _asmy_character_in_c_anim_blueprint true)))

(fn ConstructionScript)

(fn CheckIsDead
  ;[1 1 1] -Checks if Health is <=0 and shows Mission Failed in UI
  (if (<= (Variables|Default|GetHealth) 0.0)
    (Default|ShowMissionFailed (Variables|Default|GetUIPlayer))
    (Variables|Default|SetIsDead true)))