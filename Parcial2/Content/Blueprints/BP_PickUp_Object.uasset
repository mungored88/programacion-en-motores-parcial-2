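; BP_PickUp_Object is a health pickup that squashes and orients itself on BeginPlay, then spins by a fixed step every tick.
; When BP_My_Character_In_C_ok overlaps its static mesh, it adds clamped health and refreshes that character's health UI.
; It then spawns an explosion effect and pickup sound before destroying itself.
; A score-update call is present but never runs.
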(event OnComponentBeginOverlap(StaticMesh)
  (params (OverlappedComponent :type Primitive%20Component%20Object%20Reference) (OtherActor :type Actor%20Object%20Reference) (OtherComp :type Primitive%20Component%20Object%20Reference) (OtherBodyIndex :type Integer) (bFromSweep :type Boolean) (SweepResult :type Hit%20Result%20Structure%20%28by%20ref%29))
  ;[0.8366 0.4797 1] -Pick up Events
  (bind _asbp_my_character_in_c_ok (Utilities|Casting|CastToBP_My_Character_In_C_ok OtherActor))
  (bind _output_get (Variables|/Game/Blueprints/BP_My_Character_In_C_ok.BP_My_Character_In_C_ok_C|SetHealth _asbp_my_character_in_c_ok (Math|Float|Clamp(Float) (+ (Variables|/Game/Blueprints/BP_My_Character_In_C_ok.BP_My_Character_In_C_ok_C|GetHealth _asbp_my_character_in_c_ok) 1e+01) 0.0 1e+02)))
  (Default|UpdateHealth (Variables|/Game/Blueprints/BP_My_Character_In_C_ok.BP_My_Character_In_C_ok_C|GetUIPlayer _asbp_my_character_in_c_ok) _output_get)
  ;;[1 1 1] Particle
  (Effects|SpawnEmitteratLocation "/Game/StarterContent/Particles/P_Explosion.P_Explosion" (Transformation|GetActorLocation))
  ;;[1 1 1] Sound
  (Audio|SpawnSoundatLocation "/Engine/VREditor/Sounds/UI/Object_PickUp.Object_PickUp" (Transformation|GetActorLocation) "0, 0, 0" 1.0 1.0 0.0 0 0)
  (Actor|DestroyActor))

(event EventBeginPlay
  (Transformation|SetActorScale3D "0.800000,0.800000,0.120000")
  (Transformation|SetActorRotation "90.000000, 0, 0"))

(event Collision|EventActorBeginOverlap
  (params (OtherActor :type Actor%20Object%20Reference)))

(event EventTick
  (params (DeltaSeconds :type Float%20%28single-precision%29))
  ;[1 0.6367 0.5667] -Object Rotation
  (Transformation|AddActorLocalRotation "0.000000,0.000000,4.000000" false false))

(fn ConstructionScript)