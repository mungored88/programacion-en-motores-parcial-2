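; Player character Blueprint for a zombie shooter, with a socket-attached gun, health and a score/life HUD widget.
; Damage lowers clamped health and updates the HUD; Tick checks for death, shows mission failed and opens the menu after a delay.
; Line-trace shooting that damages BP_Zombie1 and sound-timed magazine reloading are present, but no event triggers either, so neither runs.
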(event Custom|Damage
  (params (Receive_damage :type Float%20%28single-precision%29))
  (bind _uiplayer (Variables|Default|GetUIPlayer))
  ;[1 0.6277 0.6509] -Receive Damage
  (Variables|Default|SetHealth (Math|Float|Clamp(Float) (- (Variables|Default|GetHealth) Receive_damage) 0.0 1e+02))
  (Default|UpdateHealth _uiplayer (Variables|Default|GetHealth))
  (Default|ShowGetDamage _uiplayer))

(event EventBeginPlay
  ;[0.1378 0.4947 1] -Create and show Score widget
  (Utilities|FlowControl|Sequence
    (:then_0
      (bind _returnvalue (UserInterface|CreateWidget "/Game/UI/UI_ScoreLife.UI_ScoreLife_C"))
      (bind _output_get (Variables|Default|SetUIPlayer _returnvalue))
      (UserInterface|Viewport|AddtoViewport _output_get 0)
      (Default|UpdateAmmo _output_get (Variables|Default|GetBulletMagazine)))
    (:then_1
      (Transformation|AttachComponentToComponent (Variables|Default|GetGun) (Variables|Character|GetMesh) "Weapon" "SnapToTarget" "KeepRelative" "KeepRelative" true))))

(event EventTick
  (params (DeltaSeconds :type Float%20%28single-precision%29))
  ;[1 0.1512 0.2878] -Is Dead?
  (CallFunction|CheckIsDead)
  (if (Variables|Default|GetIsDead)
    (Utilities|FlowControl|Delay 5.0)
    (Game|OpenLevel(byName) "Menu")))

(event Collision|EventActorBeginOverlap
  (params (OtherActor :type Actor%20Object%20Reference)))

(event Input|AxisEvents|InputAxisMouseX
  (params (AxisValue :type Float%20%28single-precision%29))
  (Pawn|Input|AddControllerYawInput AxisValue))

(event Input|MouseEvents|LeftMouseButton
  (params (Key :type Key%20Structure :default "None"))
  ;[1 0.03438 0.02775] -Shoot
)

(fn ConstructionScript)

(fn CheckIsDead
  ;[1 1 1] -Checks if Health is <=0 and shows Mission Failed in UI
  (if (<= (Variables|Default|GetHealth) 0.0)
    (Default|ShowMissionFailed (Variables|Default|GetUIPlayer))
    (Variables|Default|SetIsDead true)))