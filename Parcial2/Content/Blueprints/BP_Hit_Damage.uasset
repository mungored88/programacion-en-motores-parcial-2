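; BP_Hit_Damage is a short-lived hitbox actor that damages the player character class and destroys itself 0.3 seconds after BeginPlay.
; A Box overlap casts to BP_My_Character_In_C_ok, waits 0.2 seconds, then calls its Damage function and destroys the actor.
; When the Impulse flag is set, Tick prints a debug string and adds a fixed world-space knockback to that cast character before the same damage-and-destroy step.
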(event OnComponentBeginOverlap(Box)
  (params (OverlappedComponent :type Primitive%20Component%20Object%20Reference) (OtherActor :type Actor%20Object%20Reference) (OtherComp :type Primitive%20Component%20Object%20Reference) (OtherBodyIndex :type Integer) (bFromSweep :type Boolean) (SweepResult :type Hit%20Result%20Structure%20%28by%20ref%29))
  (bind _asbp_my_character_in_c_ok (Utilities|Casting|CastToBP_My_Character_In_C_ok OtherActor))
  (Utilities|FlowControl|Delay 0.2)
  (Default|Damage _asbp_my_character_in_c_ok (Variables|Components|GetDamages))
  (Actor|DestroyActor))

(event EventBeginPlay
  (Utilities|FlowControl|Delay 0.3)
  (Actor|DestroyActor))

(event EventTick
  (params (DeltaSeconds :type Float%20%28single-precision%29))
  (if (Variables|Components|GetImpulse)
    (Development|PrintString "Hello")
    (Physics|AddImpulse (Variables|/Script/Engine.Character|GetCharacterMovement (stale OnComponentBeginOverlap(Box) _asbp_my_character_in_c_ok)) "-3000.000000,0.000000,500.000000" true)
    (Default|Damage (stale OnComponentBeginOverlap(Box) _asbp_my_character_in_c_ok) (Variables|Components|GetDamages))
    (Actor|DestroyActor)))

(fn ConstructionScript)