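; Obstacle spawner Blueprint that periodically spawns an enemy at one of three arrow-marked positions while active.
; On BeginPlay it caches the arrow locations and looks up the maximum spawn delay from a map keyed by the game instance's difficulty.
; Tick drives a randomized Delay as a repeating timer, then spawns the Enemies class at a randomly picked cached position.
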(event EventBeginPlay
  (bind _position (Variables|Default|GetPosition))
  (Utilities|Array|Add _position (Transformation|GetWorldLocation (Variables|Default|GetArrow)))
  (Utilities|Array|Add _position (Transformation|GetWorldLocation (Variables|Default|GetArrow1)))
  (Utilities|Array|Add _position (Transformation|GetWorldLocation (Variables|Default|GetArrow2)))
  (bind _asdificultad_level_intance (Utilities|Casting|CastToDificultadLevelIntance (Game|GetGameInstance)))
  (Variables|Default|SetRandomFloat1 (.Value (Utilities|Map|Find (Variables|Default|GetMapaRandomFloat1) (Variables|/Game/MenuStaff/Dificultades/DificultadLevelIntance.DificultadLevelIntance_C|GetDificultad _asdificultad_level_intance)))))

(event EventTick
  (params (DeltaSeconds :type Float%20%28single-precision%29))
  (if (Variables|Default|GetIsActive)
    (Utilities|FlowControl|Delay (Math|Random|RandomFloatinRange 1e+01 (Variables|Default|GetRandomFloat1)))
    (Game|SpawnActorfromClass (Variables|Default|GetEnemies) (Math|Transform|MakeTransform (Utilities|Array|Get(acopy) (Variables|Default|GetPosition) (Math|Random|RandomIntegerinRange 0 2)) "0, 0, 0" "1,1,1") "Undefined" 0 0)))

(fn ConstructionScript)